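; VR brush actor, parented to the player pawn, that stamps triangle meshes into the world.
; On BeginPlay it binds to the player controller's trigger and scale events, then takes its parent's owner after a short delay.
; Each trigger press spawns a replicated generic Actor with a runtime-added, shadowless triangle mesh at the brush transform and scale.
; Scale input nudges the preview triangle's X and Y with crossed axes and a minimum-size check.
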(event Custom|OnBrushTriggerPressed
  (bind _scene (Variables|Default|GetScene))
  (bind _returnvalue (Transformation|GetWorldTransform _scene))
  (bind (_location _rotation) (Math|Transform|BreakTransform _returnvalue))
  (Development|PrintString "Brush Trigger Pressed")
  (bind _returnvalue_2 (Game|SpawnActorfromClass "/Script/Engine.Actor" _returnvalue "AlwaysSpawn" 0 0))
  (bind _returnvalue_3 (AddComponent|AddStaticMeshComponent _returnvalue_2 false (Math|Transform|MakeTransform _location _rotation "0.100000,0.100000,0.100000")))
  (Components|StaticMesh|SetStaticMesh _returnvalue_3 "/Game/Player/Brush/Triangle/Meshes/triangle1.triangle1")
  (Rendering|SetCastShadow _returnvalue_3 false)
  (Transformation|SetWorldScale3D _returnvalue_3 (Transformation|GetWorldScale (Variables|Default|GetTriangle)))
  (Networking|SetReplicates _returnvalue_2 true))

(event Custom|OnScale
  (params (ScaleX :type Float%20%28single-precision%29) (ScaleY :type Float%20%28single-precision%29))
  (bind _triangle (Variables|Default|GetTriangle))
  (bind _returnvalue (Transformation|GetWorldScale _triangle))
  (Development|PrintString (Utilities|String|Append "ScaleBrush" "     " (Utilities|String|ToString(Float) 0.0)))
  (Utilities|FlowControl|Sequence
    (:then_0
      (Transformation|SetWorldScale3D _triangle (Math|Vector|MakeVector (select (>= (.x _returnvalue) 0.02) (+ (* ScaleY 0.001) (.x _returnvalue)) 0.02) (select (>= (.y _returnvalue) 0.02) (+ (* ScaleX 0.001) (.y _returnvalue)) 0.02) (.z _returnvalue))))))

(event EventBeginPlay
  (bind _returnvalue (Actor|GetParentActor))
  (|CallParentFunction)
  (bind _asbp_player_controller (Utilities|Casting|CastToBP_PlayerController (Game|GetPlayerController 0)))
  (EventDispatchers|BindEventtoOnBrushTriggerPressed _asbp_player_controller (EventDispatchers|CreateEvent :!event Custom|OnBrushTriggerPressed))
  (EventDispatchers|BindEventtoOnScaleBrush _asbp_player_controller (EventDispatchers|CreateEvent :!event Custom|OnScale))
  (Utilities|FlowControl|Delay 0.2)
  (Actor|SetOwner (Components|GetOwner _returnvalue))
  (bind _asbp_vrplayer_pawn (Utilities|Casting|CastToBP_VRPlayerPawn _returnvalue)))

(event Collision|EventActorBeginOverlap
  (params (OtherActor :type Actor%20Object%20Reference))
  (|CallParentFunction OtherActor) ; This node is disabled and will not be called.\nDrag off pins to build functionality.
)

(event EventTick
  (params (DeltaSeconds :type Float%20%28single-precision%29))
  (|CallParentFunction DeltaSeconds))

(fn ConstructionScript
  (|CallParentFunction))