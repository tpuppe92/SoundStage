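; Player controller for a multiplayer VR brush-and-palette app, handling input, locomotion and session hosting/finding through BP_SoundStageGameInstance.
; Triggers map to brush or palette by handedness and fire event dispatchers, with brush presses and joystick scaling routed through server events.
; Locally, it moves BP_VRPlayerPawn by axis offsets relative to headset or control rotation, plus a grab-style drag from the brush controller's pressed position, drawn with a debug arrow.
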(event Custom|Server_BrushTriggerPressed
  (Default|CallOnBrushTriggerPressed))

(event Custom|Server_BrushTriggerReleased
  (Default|CallOnBrushTriggerReleased))

(event Custom|Server_ScaleEvent
  (params (ScaleX :type Float%20%28single-precision%29) (ScaleY :type Float%20%28single-precision%29))
  (Default|CallOnScaleBrush ScaleX ScaleY))

(event EventBeginPlay)

(event EventTick
  (params (DeltaSeconds :type Float%20%28single-precision%29)))

(event Input|ActionEvents|InputActionRightControllerTrigger
  (params (Key :type Key%20Structure :default "None"))
  (bind _isrighthanded (Variables|Default|GetIsRightHanded))
  (:Pressed
    (if _isrighthanded
      (CallFunction|ServerBrushTriggerPressed)
      (else
        (Default|CallOnPaletteTriggerPressed))))
  (:Released
    (if _isrighthanded
      (CallFunction|ServerBrushTriggerReleased)
      (else
        (Default|CallOnPaletteTriggerReleased)))))

(event Input|ActionEvents|InputActionLeftControllerTrigger
  (params (Key :type Key%20Structure :default "None"))
  (bind _isrighthanded (Variables|Default|GetIsRightHanded))
  (:Pressed
    (if _isrighthanded
      (Default|CallOnPaletteTriggerPressed)
      (else
        (CallFunction|ServerBrushTriggerPressed))))
  (:Released
    (if _isrighthanded
      (Default|CallOnPaletteTriggerReleased)
      (else
        (CallFunction|ServerBrushTriggerReleased)))))

(event Input|ActionEvents|InputActionHost
  (params (Key :type Key%20Structure :default "None"))
  (:Pressed
    (bind _asbp_sound_stage_game_instance (Utilities|Casting|CastToBP_SoundStageGameInstance (Game|GetGameInstance))
      (:then
        (Class|SoundStageGameInstance|Host _asbp_sound_stage_game_instance "SoundStageGameSession")
        (Development|PrintString "Host"))
      (:CastFailed
        (Development|PrintString "Host Cast Failed!!!!!!!")))))

(event Input|ActionEvents|InputActionFind
  (params (Key :type Key%20Structure :default "None"))
  (:Pressed
    (bind _asbp_sound_stage_game_instance (Utilities|Casting|CastToBP_SoundStageGameInstance (Game|GetGameInstance))
      (:then
        (Class|SoundStageGameInstance|FindSessions _asbp_sound_stage_game_instance)
        (Development|PrintString "Find"))
      (:CastFailed
        (Development|PrintString "Host Cast Failed!!!!!!!")))))

(event Input|ActionEvents|InputActionMove
  (params (Key :type Key%20Structure :default "None"))
  (:Pressed
    (if (Pawn|IsLocalController)
      (bind _asbp_vrplayer_pawn (Utilities|Casting|CastToBP_VRPlayerPawn (Pawn|GetControlledPawn)))
      (Variables|Default|SetStartMoveVector (Transformation|GetWorldLocation (Variables|/Game/Player/Blueprints/BP_VRPlayerPawn.BP_VRPlayerPawn_C|GetBrushMotionController _asbp_vrplayer_pawn)))
      (Development|PrintString "A button")
      (Variables|Default|SetStartActorLocation (Transformation|GetActorLocation _asbp_vrplayer_pawn)))))

(event Input|AxisEvents|InputAxisMoveForward
  (params (AxisValue :type Float%20%28single-precision%29))
  (if (Pawn|IsLocalController)
    (if (> (Math|Float|Absolute(Float) AxisValue) 0.1)
      (bind _asbp_vrplayer_pawn (Utilities|Casting|CastToBP_VRPlayerPawn (Pawn|GetControlledPawn)))
      (Transformation|AddActorWorldOffset _asbp_vrplayer_pawn (* (select (Class|HeadMountedDisplayFunctionLibrary|IsHeadMountedDisplayEnabled) (Math|Vector|GetForwardVector (Variables|/Game/Player/Blueprints/BP_VRPlayerPawn.BP_VRPlayerPawn_C|GetCamera _asbp_vrplayer_pawn)) (Math|Vector|Normalize (* (Math|Vector|GetForwardVector (Pawn|GetControlRotation :!class /Script/Engine.Controller)) "1.000000,1.000000, 0"))) (* AxisValue (Variables|Default|GetMovementSpeed)))))))

(event Input|AxisEvents|InputAxisMoveRight
  (params (AxisValue :type Float%20%28single-precision%29))
  (if (Pawn|IsLocalController)
    (if (> (Math|Float|Absolute(Float) AxisValue) 0.1)
      (bind _asbp_vrplayer_pawn (Utilities|Casting|CastToBP_VRPlayerPawn (Pawn|GetControlledPawn)))
      (Transformation|AddActorWorldOffset _asbp_vrplayer_pawn (* (select (Class|HeadMountedDisplayFunctionLibrary|IsHeadMountedDisplayEnabled) (Math|Vector|GetRightVector (Variables|/Game/Player/Blueprints/BP_VRPlayerPawn.BP_VRPlayerPawn_C|GetCamera _asbp_vrplayer_pawn)) (Math|Vector|Normalize (* (Math|Vector|GetRightVector (Pawn|GetControlRotation :!class /Script/Engine.Controller)) "1.000000,1.000000, 0"))) (* AxisValue (Variables|Default|GetMovementSpeed)))))))

(event Input|AxisEvents|InputAxisMoveUp
  (params (AxisValue :type Float%20%28single-precision%29))
  (if (Pawn|IsLocalController)
    (if (> (Math|Float|Absolute(Float) AxisValue) 0.1)
      (bind _asbp_vrplayer_pawn (Utilities|Casting|CastToBP_VRPlayerPawn (Pawn|GetControlledPawn)))
      (Transformation|AddActorWorldOffset _asbp_vrplayer_pawn (* "0, 0,1.000000" (* AxisValue (Variables|Default|GetMovementSpeed)))))))

(event Input|AxisEvents|InputAxisMoveController
  (params (AxisValue :type Float%20%28single-precision%29))
  (if (Pawn|IsLocalController)
    (if (> (Math|Float|Absolute(Float) AxisValue) 0.1)
      (bind _asbp_vrplayer_pawn (Utilities|Casting|CastToBP_VRPlayerPawn (Pawn|GetControlledPawn)))
      (Pawn|Input|AddMovementInput _asbp_vrplayer_pawn (- (+ (Variables|Default|GetStartMoveVector) (- (Transformation|GetActorLocation _asbp_vrplayer_pawn) (Variables|Default|GetStartActorLocation))) (Transformation|GetWorldLocation (Variables|/Game/Player/Blueprints/BP_VRPlayerPawn.BP_VRPlayerPawn_C|GetBrushMotionController _asbp_vrplayer_pawn))) 1.0 false)
      (Rendering|Debug|DrawDebugArrow (+ (Variables|Default|GetStartMoveVector) (- (Transformation|GetActorLocation _asbp_vrplayer_pawn) (Variables|Default|GetStartActorLocation))) (Transformation|GetWorldLocation (Variables|/Game/Player/Blueprints/BP_VRPlayerPawn.BP_VRPlayerPawn_C|GetBrushMotionController _asbp_vrplayer_pawn)) 1.0 "(R=0.447405,G=0.107781,B=0.578125,A=1.000000)" 0.0 1.0))))

(event Input|AxisEvents|InputAxisTurn
  (params (AxisValue :type Float%20%28single-precision%29))
  (if (Pawn|IsLocalController)
    (if (> (Math|Float|Absolute(Float) AxisValue) 0.1)
      (bind _asbp_vrplayer_pawn (Utilities|Casting|CastToBP_VRPlayerPawn (Pawn|GetControlledPawn)))
      (Pawn|Input|AddControllerYawInput _asbp_vrplayer_pawn AxisValue))))

(event Input|AxisEvents|InputAxisLookUp
  (params (AxisValue :type Float%20%28single-precision%29))
  (if (Pawn|IsLocalController)
    (if (> (Math|Float|Absolute(Float) AxisValue) 0.1)
      (bind _asbp_vrplayer_pawn (Utilities|Casting|CastToBP_VRPlayerPawn (Pawn|GetControlledPawn)))
      (Pawn|Input|AddControllerPitchInput _asbp_vrplayer_pawn AxisValue))))

(event Input|AxisEvents|InputAxisScaleBrush
  (params (AxisValue :type Float%20%28single-precision%29))
  (bind _returnvalue (Input|AxisValues|GetRightControllerJoystickY))
  (bind _returnvalue_2 (Input|AxisValues|GetRightControllerJoystickX))
  (if (or (> (Math|Float|Absolute(Float) _returnvalue_2) 0.1) (> (Math|Float|Absolute(Float) _returnvalue) 0.1))
    (CallFunction|ServerScaleEvent _returnvalue_2 _returnvalue)))

(fn ConstructionScript)