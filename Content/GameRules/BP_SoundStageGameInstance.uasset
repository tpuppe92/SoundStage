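; Game instance for SoundStage that joins an online session when one is found.
; The find-session event sets a found flag and joins the session at the reported index.
; Init only prints a debug message.
; Delayed chains to search for sessions, or host a SoundStage session if none is found, exist but are disconnected and never run.
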(event EventBIEonFindSession
  (params (idx :type Integer))
  (Development|PrintString "Found Sesseion")
  (Variables|Default|SetbSessionIsFound true)
  (Class|SoundStageGameInstance|JoinSession idx))

(event EventInit
  (Development|PrintString "BP GameInstance   diggggggiii!!!!"))